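; BPC_CellMoveComponent is a movement component that spins and linearly moves its owning cell actor.
; Each tick applies yaw at angular speed minus drag, and while active offsets the actor along a direction at linear speed minus drag, both clamped at zero.
; LinerMove sets the direction and enables translation for a given duration.
; Steps are not scaled by delta time or swept, and the looping-timer alternative is unconnected.
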(event Custom|LinerMove
  (params (LinerVelocityDirection :type Vector) (Duration :type Float%20%28single-precision%29))
  (CallFunction|StartMove)
  (Variables|Default|SetLinerVelocityDirection LinerVelocityDirection)
  (Utilities|FlowControl|Delay Duration)
  (CallFunction|StopMove))

(event Custom|StartMove
  (Variables|Default|SetbIsActiveMove true))

(event Custom|MoveOnTick
  (bind _angularspeed (Variables|Default|GetAngularSpeed))
  (bind _linerdrag (Variables|Default|GetlinerDrag))
  (bind _angulardrag (Variables|Default|GetAngularDrag))
  (bind _linervelocityspeed (Variables|Default|GetLinerVelocitySpeed))
  (bind _returnvalue (- _linervelocityspeed _linerdrag))
  (bind _returnvalue_2 (- _angularspeed _angulardrag))
  (Utilities|FlowControl|Sequence
    (:then_0
      (Transformation|AddActorLocalRotation (Components|GetOwner) (Math|Rotator|MakeRotator 0.0 0.0 (Math|Float|SelectFloat _returnvalue_2 0.0 (>= _returnvalue_2 0.0))) false false))
    (:then_1
      (if (Variables|Default|GetbIsActiveMove)
        (Transformation|AddActorWorldOffset (Components|GetOwner) (* (Math|Float|SelectFloat _returnvalue 0.0 (>= _returnvalue 0.0)) (Variables|Default|GetLinerVelocityDirection)))))))

(event Custom|StopMove
  (Variables|Default|SetbIsActiveMove false))

(event EventTick
  (params (DeltaSeconds :type Float%20%28single-precision%29))
  (bind _angularspeed (Variables|Default|GetAngularSpeed))
  (bind _linerdrag (Variables|Default|GetlinerDrag))
  (bind _angulardrag (Variables|Default|GetAngularDrag))
  (bind _linervelocityspeed (Variables|Default|GetLinerVelocitySpeed))
  (bind _returnvalue (- _linervelocityspeed _linerdrag))
  (bind _returnvalue_2 (- _angularspeed _angulardrag))
  (Utilities|FlowControl|Sequence
    (:then_0
      (Transformation|AddActorLocalRotation (Components|GetOwner) (Math|Rotator|MakeRotator 0.0 0.0 (Math|Float|SelectFloat _returnvalue_2 0.0 (>= _returnvalue_2 0.0))) false false))
    (:then_1
      (if (Variables|Default|GetbIsActiveMove)
        (Transformation|AddActorWorldOffset (Components|GetOwner) (* (Math|Float|SelectFloat _returnvalue 0.0 (>= _returnvalue 0.0)) (Variables|Default|GetLinerVelocityDirection)))))))