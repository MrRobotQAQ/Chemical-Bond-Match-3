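; BP_CellBase is a cell actor, apparently a base class, that drifts around the level on its own.
; On BeginPlay it makes a linear move toward player 0's position at that moment, then loops random X/Y nudges separated by one-second delays.
; BPCCellMoveComponent performs the movement through LinerMove, given a direction and duration.
; A similar MoveComponentTo version remains in the graph but is disconnected.
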(event Custom|MoveOnStart
  (bind _returnvalue (Math|Random|RandomUnitVector))
  (bind (_x _y) (Math|Vector|BreakVector _returnvalue))
  (Default|LinerMove (Variables|Default|GetBPC_CellMoveComponent) (Math|Vector|Normalize (- (Transformation|GetActorLocation (Game|GetPlayerCharacter 0)) (Transformation|GetActorLocation))) 1.0)
  (Utilities|FlowControl|Delay 1.0 :!label _label)
  (Default|LinerMove (Variables|Default|GetBPC_CellMoveComponent) (Math|Vector|MakeVector _x _y 0.0) 0.5)
  (goto _label))

(event EventBeginPlay
  (CallFunction|MoveonStart))

(fn ConstructionScript)